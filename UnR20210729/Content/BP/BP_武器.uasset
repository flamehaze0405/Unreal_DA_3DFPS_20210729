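; Weapon Blueprint that provides automatic fire and magazine reloading.
; While the fire input (開槍攻擊) is held and rounds remain, a Delay loop spawns BP_子彈 and a muzzle flash at the 子彈插槽 socket, spending one round per shot at the 開槍間隔 interval.
; Custom event 換彈夾, not called within this Blueprint, refills the magazine from the reserve total, limited to what remains.
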(event `InputAction|開槍攻擊`
  (params (Key :type "Key Structure"))
  (bind `_武器模型` (`self.武器模型`))
  (bind (_returnvalue_roll _returnvalue_pitch _returnvalue_yaw) (`KismetMathLibrary.BreakRotator` (`SceneComponent.GetSocketRotation` `_武器模型` "子彈插槽")))
  ;[1 1 1] 開槍功能
  (:`Pressed`
    (set `self.開槍中` true)
    (if (and (> (`self.目前子彈數量`) 0) (`self.開槍中`)) :!label _label
      (`|SpawnActorFromClass` "/Game/BP/BP_子彈.BP_子彈_C" (`SceneComponent.GetSocketTransform` (`self.武器模型`) "子彈插槽" "RTS_World") "Undefined" "OverrideRootScale" null null) ; 生成子彈藍圖
      (`GameplayStatics.SpawnEmitterAtLocation` "/Game/InfinityBladeEffects/Effects/FX_Monsters/FX_Monster_Gruntling/Master/P_BackPack_MuzzleFlash.P_BackPack_MuzzleFlash" (`SceneComponent.GetSocketLocation` `_武器模型` "子彈插槽") (`KismetMathLibrary.MakeRotator` (+ _returnvalue_roll 90.0) (+ _returnvalue_pitch -10.0) (+ _returnvalue_yaw 0.0)) (0.05 0.05 0.05))
      (set `self.目前子彈數量` (- (`self.目前子彈數量`) 1))
      (`KismetSystemLibrary.Delay` (`self.開槍間隔`))
      (goto _label)))
  (:`Released`
    (set `self.開槍中` false)))

(event `換彈夾`
  ;[1 1 1] 換彈夾
  ;;[0.6432 1 0.5073] 計算要補充幾顆子彈
  (set `self.要補充的子彈數量` (- (`self.彈夾尺寸`) (`self.目前子彈數量`))) ; 計算要補充的子彈數量，\n例 : 目前10彈夾30所以要補充20
  ;;[1 0.8767 0.2531] 判斷總數是否>=要補充的數量
  (if (not (>= (`self.子彈總數`) (`self.要補充的子彈數量`)))
    ;;[1 1 1] 總數<要補充的數量 : 把剩於總數補充
    (set `self.要補充的子彈數量` (`self.子彈總數`)))
  ;;[1 1 1] 總數>=要補充的數量
  (set `self.目前子彈數量` (+ (`self.目前子彈數量`) (`self.要補充的子彈數量`))) ; 補充子彈數量，例 : 目前10要補充為20補充後為30
  ;;[1 1 1] 目前子彈及總數更新
  (set `self.子彈總數` (- (`self.子彈總數`) (`self.要補充的子彈數量`))) ; 扣除子彈總數，例 : 總數為20要補充為20補充後總數為0
)

(fn `UserConstructionScript`)