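; Game mode Blueprint that runs a minute-and-second countdown timer and pauses the game when time runs out.
; Event Tick feeds a one-second Delay, so the seconds variable (秒) drops by one roughly every second rather than every frame.
; When seconds fall below zero they wrap to 59 and minutes (分) decrease; with no minutes left, seconds reset to zero and the game pauses.
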(event `self.ReceiveTick`
  (params (DeltaSeconds :type "Float (single-precision)"))
  ;[0.1354 0.1354 0.1354] 時間倒數系統
  ;;[1 0.1159 0.6233] 每秒倒數1
  (`KismetSystemLibrary.Delay` 1.0) ; 延遲 : 等待所設定的時間
  (bind _output_get (set `self.秒` (- (`self.秒`) 1)))
  ;;[1 0.1978 0.2078] 秒數低於0就設為59
  (if (< _output_get 0)
    (set `self.秒` 59)
    ;;[1 1 1] 分大於0時分減1
    (if (> (`self.分`) 0)
      (set `self.分` (- (`self.分`) 1))
      (else
        ;;[1 1 1] 分為0時，秒等於59，就代表時間歸0，遊戲無法繼續進行
        (if (== (`self.秒`) 59)
          (set `self.秒` 0)
          (`GameplayStatics.SetGamePaused` true))))))

(fn `UserConstructionScript`)