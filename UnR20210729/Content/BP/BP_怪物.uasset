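; Monster enemy that wanders randomly, chases the player and melee-attacks, using a looping AIMoveTo flow instead of a behavior tree.
; Pawn sensing or a non-lethal bullet hit sets the chase flag.
; Reaching the player stops movement and briefly enables the attack zone's overlap events on timed delays to deal damage.
; Bullet overlaps drain health; death ragdolls the mesh, increments the game mode's kill count and destroys the actor after a delay.
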(event `self.ReceiveBeginPlay`
  (bind _charactermovement (`self.CharacterMovement`))
  (bind `_攻擊區域` (`self.攻擊區域`))
  (`|ExecutionSequence`
    (:`then_0`
      (if (`self.是否看到玩家`) :!label _label
        ;[1 0.3737 0.3538] 看到玩家以及失去玩家蹤跡的事件
        (`|AIMoveTo` self (0.0 0.0 0.0) (`self.As BP 玩家控制`) (`self.停止半徑`) ; 看到玩家
          (:`OnSuccess`
            ;[1 0.1567 0.4095] 攻擊狀態
            (set `self.攻擊中` true)
            (set `CharacterMovementComponent.MaxWalkSpeed` 0.0 _charactermovement)
            (`KismetSystemLibrary.Delay` 1.5) ; 攻擊動畫中無效判定時間
            (set `PrimitiveComponent.bGenerateOverlapEvents` true `_攻擊區域`)
            (`KismetSystemLibrary.Delay` 0.2) ; 攻擊判定
            (set `PrimitiveComponent.bGenerateOverlapEvents` false `_攻擊區域`)
            (`KismetSystemLibrary.Delay` 1.67)
            (set `CharacterMovementComponent.MaxWalkSpeed` 600.0 _charactermovement)
            (set `self.攻擊中` false)
            (goto _label))
          (:`OnFail`
            (set `self.是否看到玩家` false)
            (set `self.停留時最大值` 3.0)
            (goto _label)))
        (else
          ;[0.2572 0.7246 1] AI隨機移動事件
          (`|AIMoveTo` self (`NavigationSystemV1.K2_GetRandomReachablePointInRadius` (`SceneComponent.K2_GetComponentLocation` (`self.CapsuleComponent`)) (`self.隨機走動半徑`) null null) null (`self.停止半徑`) ; AI移動節點
            (:`then`
              ;;[0.272 1 0.5884] 隨機停留
              (`KismetSystemLibrary.Delay` (* (`KismetMathLibrary.RandomFloat`) (`self.停留時最大值`)))
              (goto _label))))))
    (:`then_1`
      ;[1 1 1] 取得遊戲模式
      (bind `_asbp_遊戲模式` (cast `/Game/BP/BP_遊戲模式` (`GameplayStatics.GetGameMode`)))
      (set `self.遊戲模式` `_asbp_遊戲模式`))))

(event `self.感測元件.OnSeePawn`
  (params (Pawn :type "Pawn Object Reference"))
  ;[0.9147 0.1327 1] 怪物視線偵測
  (bind `_asbp_玩家控制` (cast `/Game/BP/BP_玩家控制` Pawn))
  (set `self.As BP 玩家控制` `_asbp_玩家控制`)
  (set `self.是否看到玩家` true :!label _label_2)
  (set `self.停留時最大值` 0.0) ; 看見玩家時停留時間
  (`/Engine/EditorBlueprintResources/StandardMacros.DoOnce` false ; 執行一次
    (:`Completed`
      (goto _label))))

(event `self.CapsuleComponent.OnComponentBeginOverlap`
  (params (OverlappedComponent :type "PrimitiveComponent Object Reference") (OtherActor :type "Actor Object Reference") (OtherComp :type "PrimitiveComponent Object Reference") (OtherBodyIndex :type Integer) (bFromSweep :type Boolean) (SweepResult :type "HitResult Structure (by ref)"))
  (bind `_遊戲模式` (`self.遊戲模式`))
  ;[1 0.1198 0.1198] 受傷與死亡
  (bind `_asbp_子彈` (cast `/Game/BP/BP_子彈` OtherActor))
  (bind `_是否死亡` (`self.受傷` (`/Game/BP/BP_子彈.傷害值` `_asbp_子彈`)))
  (if `_是否死亡`
    (set `/Game/BP/BP_遊戲模式.擊殺怪物數量` (+ (`/Game/BP/BP_遊戲模式.擊殺怪物數量` `_遊戲模式`) 1) `_遊戲模式`)
    (`KismetSystemLibrary.Delay` 5.0)
    (`self.K2_DestroyActor`)
    (else
      (goto _label_2))))

(event `self.攻擊區域.OnComponentBeginOverlap`
  (params (OverlappedComponent :type "PrimitiveComponent Object Reference") (OtherActor :type "Actor Object Reference") (OtherComp :type "PrimitiveComponent Object Reference") (OtherBodyIndex :type Integer) (bFromSweep :type Boolean) (SweepResult :type "HitResult Structure (by ref)"))
  ;[1 1 1] 攻擊區域
  (bind `_asbp_玩家控制` (cast `/Game/BP/BP_玩家控制` OtherActor))
  (`/Game/BP/BP_玩家控制.受傷` `_asbp_玩家控制` (`self.怪物攻擊力`)))

(fn `UserConstructionScript`)

(fn `受傷`
  (params (`接收到傷害值` :type "Float (double-precision)"))
  (returns (`是否死亡` :type Boolean))
  (bind _output_get (set `self.血量` (- (`self.血量`) `接收到傷害值`)))
  (if (<= _output_get 0.0)
    (`PrimitiveComponent.SetSimulatePhysics` (`self.Mesh`) true) ; 模擬布偶效果
    (`PrimitiveComponent.SetCollisionEnabled` (`self.CapsuleComponent`) "NoCollision") ; 設定碰撞的啟動 : 關閉膠囊碰撞避免產生太大變化
    (return true)
    (else
      (return false))))